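; Actor that runs a socket client session with a CVM server at a hard-coded IP and port.
; On BeginPlay it connects, sends CP message 202 and shows a Discon widget that receives the socket, which is closed when the actor is destroyed.
; Tick polls for pending data and runs ProcessMSG, with events for numbered incoming messages.
; Only the 82 and 108 handlers act, printing debug text; 101, 112 and 123 are empty.
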(event `self.ReceiveBeginPlay`
  (bind (_success _returnvalue) (`SocketerBPLibrary.Connect` "192.168.240.112" 21223))
  (if _success
    (set `self.soket` _returnvalue)
    (`KismetSystemLibrary.PrintString` "connected")
    (`self.SendCPMsg202` _returnvalue)
    (bind _returnvalue_2 (`|CreateWidget` "/Game/Assets/UMG/discon.discon_C" (`GameplayStatics.GetPlayerController` 0)))
    (set `/Game/Assets/UMG/discon.soc` (`self.soket`) _returnvalue_2)
    (`UserWidget.AddToViewport` _returnvalue_2 0)))

(event `self.ReceiveDestroyed`
  (`SocketerBPLibrary.CloseConnection` (`self.soket`)))

(event `self.ReceiveTick`
  (params (DeltaSeconds :type "Float (single-precision)"))
  (bind _soket (`self.soket`))
  (if (`SocketerBPLibrary.HasPendingData` _soket)
    (bind _messagecome (`self.processMSG` _soket))))

(event `self.Message_123_Come`
  (params (msg :type "BPCPMsg123 Structure")))

(event `self.Message_82_Come`
  (params (msg :type "BPCPMsg82 Structure"))
  (`KismetSystemLibrary.PrintString` "message 82!!!!!!!"))

(event `self.Message_112_Come`
  (params (msg :type "BPCPMsg112 Structure")))

(event `self.Message_101_Come`
  (params (msg :type "BPCPMsg101 Structure")))

(event `self.Message_108_Come`
  (params (msg :type "BPCPMsg108 Structure"))
  (`KismetSystemLibrary.PrintString` (`KismetStringLibrary.Conv_IntToString` (`.NumAb` (break `BPCPMsg108` msg)))))

(fn `UserConstructionScript`)